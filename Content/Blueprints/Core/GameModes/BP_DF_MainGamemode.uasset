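; Main game mode that takes over pawn spawning and possession for joining players.
; SpawnDefaultPawnFor returns no pawn, leaving PostLogin to spawn and possess one.
; If player character 0 exists, an EQS query runs from it and the new pawn spawns at a random result location.
; Otherwise, the pawn spawns at the first PlayerStart found.
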(event `self.K2_PostLogin`
  (params (NewPlayer :type "PlayerController Object Reference"))
  (bind _returnvalue (`GameplayStatics.GetPlayerCharacter` 0))
  (`/Engine/EditorBlueprintResources/StandardMacros.IsValid` _returnvalue
    (:`Is Valid`
      (bind _returnvalue_2 (`EnvQueryManager.RunEQSQuery` null _returnvalue "RandomBest25Pct"))
      (add `EnvQueryInstanceBlueprintWrapper.OnQueryFinishedEvent` _returnvalue_2 (delegate `OnQueryFinishedEvent_Event`)))
    (:`Is Not Valid`
      (bind _outactors (`GameplayStatics.GetAllActorsOfClass` "/Script/Engine.PlayerStart"))
      (bind _returnvalue_3 (`|SpawnActorFromClass` null (`KismetMathLibrary.MakeTransform` (`self.K2_GetActorLocation` (`|GetArrayItem` _outactors))) "Undefined" "MultiplyWithRoot" null null))
      (`Controller.Possess` NewPlayer _returnvalue_3))))

(event `OnQueryFinishedEvent_Event`
  (params (QueryInstance :type "EnvQueryInstanceBlueprintWrapper Object Reference") (QueryStatus :type "EEnvQueryStatus Enum" :default "Processing"))
  (bind _resultlocations (`EnvQueryInstanceBlueprintWrapper.GetQueryResultsAsLocations` QueryInstance))
  (bind _returnvalue (`|SpawnActorFromClass` null (`KismetMathLibrary.MakeTransform` (`KismetArrayLibrary.Array_Random` _resultlocations)) "Undefined" "MultiplyWithRoot" (stale `self.K2_PostLogin` NewPlayer) null))
  (`Controller.Possess` (stale `self.K2_PostLogin` NewPlayer) _returnvalue))

(fn `SpawnDefaultPawnFor`
  (params (NewPlayer :type "Controller Object Reference") (StartSpot :type "Actor Object Reference"))
  (returns (ReturnValue :type "Pawn Object Reference"))
  (return null))

(fn `UserConstructionScript`)