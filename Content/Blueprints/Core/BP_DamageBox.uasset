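; BP_DamageBox is a damage volume that hurts an actor repeatedly while it overlaps the box.
; Begin overlap starts a looping half-second timer, and each tick sends a TakeDamage message with a fixed amount to the target's BaseAbilityComponent.
; End overlap by any actor clears the timer through its single stored handle, which each new overlap overwrites, so overlapping actors are not tracked separately.
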(event `CustomEvent`
  (params (Target :type "Actor Object Reference"))
  (bind _returnvalue (`KismetSystemLibrary.K2_SetTimerDelegate` (delegate `OnDamage`) 0.5 true))
  (set `self.DamageTimer` _returnvalue))

(event `self.Box.OnComponentBeginOverlap`
  (params (OverlappedComponent :type "PrimitiveComponent Object Reference") (OtherActor :type "Actor Object Reference") (OtherComp :type "PrimitiveComponent Object Reference") (OtherBodyIndex :type Integer) (bFromSweep :type Boolean) (SweepResult :type "HitResult Structure (by ref)"))
  (`self.CustomEvent` OtherActor))

(event `OnDamage`
  (message `DamageInterface.TakeDamage` (`self.GetComponentByClass` (stale `CustomEvent` Target) "/Script/DustFall.BaseAbilityComponent") 2.0 self "None"))

(event `self.Box.OnComponentEndOverlap`
  (params (OverlappedComponent :type "PrimitiveComponent Object Reference") (OtherActor :type "Actor Object Reference") (OtherComp :type "PrimitiveComponent Object Reference") (OtherBodyIndex :type Integer))
  (`self.CustomEvent_1`))

(event `CustomEvent_1`
  (`KismetSystemLibrary.K2_ClearAndInvalidateTimerHandle` (`self.DamageTimer`)))

(fn `UserConstructionScript`)